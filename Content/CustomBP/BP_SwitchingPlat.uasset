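; BP_SwitchingPlat is a platform that appears or disappears depending on the player character's current post-process (CurrentPPV) state.
; On BeginPlay and on Activate it hides the platform, then shows it if any ShaderType entry matches the BP_FirstPersonCharacter's CurrentPPV or is zero.
; Collision follows visibility, so hidden platforms have none and visible ones use query and physics collision.
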(event `self.ReceiveBeginPlay`
  (bind _platform (`self.Platform`))
  (`SceneComponent.SetVisibility` (`self.Platform`) false false :!label _label)
  (bind _returnvalue (`GameplayStatics.GetActorOfClass` "/Game/FirstPerson/Blueprints/BP_FirstPersonCharacter.BP_FirstPersonCharacter_C"))
  (for _array_element (`self.ShaderType`)
    (if (or (== (`/Game/FirstPerson/Blueprints/BP_FirstPersonCharacter.CurrentPPV` _returnvalue) _array_element) (== _array_element 0))
      (`SceneComponent.SetVisibility` (`self.Platform`) true false)
      (break)))
  (if (`SceneComponent.IsVisible` (`self.Platform`))
    (`PrimitiveComponent.SetCollisionEnabled` _platform "QueryAndPhysics")
    (else
      (`PrimitiveComponent.SetCollisionEnabled` _platform "NoCollision"))))

(event `Activate`
  (goto _label))

(fn `UserConstructionScript`)